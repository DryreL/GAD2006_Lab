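; BP_DamageVolume is a volume that deals continuous damage to COABaseCharacter actors overlapping it.
; Overlap begin enables actor Tick for these characters, and overlap end disables it once none remain inside.
; Each Tick applies BaseDamage scaled by delta seconds to every overlapping character, making damage per-second and frame-rate independent.
; A ModifyDamage function returns its input unchanged and is not called in these graphs.
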(event `self.ReceiveActorBeginOverlap`
  (params (OtherActor :type "Actor Object Reference"))
  (cast `COABaseCharacter` OtherActor
    (:`then`
      (`self.SetActorTickEnabled` self true))
    (:`CastFailed`
      (`KismetSystemLibrary.PrintString` "CAST FAILED!" true true (struct :`R` 1.0 :`B` 0.014468 :`A` 1.0) 5.0))))

(event `self.ReceiveActorEndOverlap`
  (params (OtherActor :type "Actor Object Reference"))
  (if (== (`KismetArrayLibrary.Array_Length` (`self.GetOverlappingActors` self "/Script/GAD2006_Lab.COABaseCharacter")) 0)
    (`self.SetActorTickEnabled` self false)))

(event `self.ReceiveTick`
  (params (DeltaSeconds :type "Float (single-precision)"))
  (for _array_element (`self.GetOverlappingActors` self "/Script/GAD2006_Lab.COABaseCharacter")
    (`/Engine/EditorBlueprintResources/StandardMacros.IsValid` _array_element
      (:`Is Valid`
        (`GameplayStatics.ApplyDamage` _array_element (* DeltaSeconds (`self.Base Damage`))))
      (:`Is Not Valid`
        (`KismetSystemLibrary.PrintString` "NOT VALID!" true true (struct :`R` 1.0 :`B` 0.014468 :`A` 1.0) 5.0)))))

(fn `ModifyDamage`
  (params (IncomingDamage :type "Float (double-precision)"))
  (returns (ReturnValue :type "Float (double-precision)"))
  (return IncomingDamage))

(fn `UserConstructionScript`)