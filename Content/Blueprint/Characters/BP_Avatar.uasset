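; Player avatar character with light and heavy sword attacks, damage reactions, death and debug aids for health printing and self-damage.
; Input and events pass state changes through Server/Multicast event pairs to ChangeAnimState, which drives the anim blueprint and slows movement and turning while attacking.
; OnAttack damages overlapping actors within a forward dot-product cone.
; AnyDamage lowers Health and updates the player controller's GUI widget through a client event.
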(event `self.ReceiveBeginPlay`
  ;[0.3229 0 0] Event BeginPlay
  (`|ExecutionSequence`
    (:`then_0`
      (bind _asanim_bp_base_character (cast `/Game/Blueprint/Characters/AnimBP_BaseCharacter` (`SkeletalMeshComponent.GetAnimInstance` (`self.Mesh`)))
        (:`then`
          (set `self.Animation` _asanim_bp_base_character)
          (`self.ChangeAnimState Server` "CAS_IDLE"))
        (:`CastFailed`
          (`KismetSystemLibrary.PrintString` "BP_Avatar - AnimBP_BaseCharacter -Cast failed!" true true (struct :`R` 1.0 :`B` 0.005787 :`A` 1.0) 5.0))))
    (:`then_1`
      (`KismetSystemLibrary.Delay` 0.5))))

(event `self.ReceiveTick`
  (params (DeltaSeconds :type "Float (single-precision)"))
  ;[0.3229 0 0] Event Tick
  (`KismetSystemLibrary.Delay` 1.0)
  (`|ExecutionSequence`
    (:`then_0`
      (`KismetSystemLibrary.PrintString` (`KismetStringLibrary.Concat_StrStr` "Health: " (`KismetStringLibrary.Conv_DoubleToString` (`self.Health`))) true true (struct :`R` 0.617198 :`G` 0.560891 :`B` 1.0 :`A` 1.0) 1.0))))

(event `InputAction|Attack`
  (params (Key :type "Key Structure"))
  ;[0.3229 0.08651 0] Event Attack/HeavyAttack
  (:`Pressed`
    (`self.AttackStyle Server` false)
    (`self.ChangeAnimState Server` "CAS_ATTACK")))

(event `self.ReceiveAnyDamage`
  (params (Damage :type "Float (single-precision)") (DamageType :type "DamageType Object Reference") (InstigatedBy :type "Controller Object Reference") (DamageCauser :type "Actor Object Reference"))
  ;[0.3229 0.08651 0] Event Anydamage
  (bind _output_get (set `self.Health` (- (`self.Health`) Damage)))
  (`KismetSystemLibrary.PrintString` (`KismetStringLibrary.Conv_DoubleToString` _output_get))
  (`self.UpdateHealth Client` _output_get))

(event `InputAction|HeavyAttack`
  (params (Key :type "Key Structure"))
  ;[0.3229 0.08651 0] Event Attack/HeavyAttack
  (:`Pressed`
    (`self.AttackStyle Server` true)
    (`self.ChangeAnimState Server` "CAS_ATTACK")))

(event `InputAction|Interact`
  (params (Key :type "Key Structure"))
  ;[0.3231 0.0865 0] E - Self Damage
  (:`Pressed`
    (bind _returnvalue (`GameplayStatics.ApplyDamage` self 5.0))
    (`KismetSystemLibrary.PrintString` (`KismetStringLibrary.Conv_DoubleToString` _returnvalue))))

(event `self.OnCharacterDied`
  ;[0.3229 0.08651 0] Event Character Died
  (`self.ChangeAnimState Server` "CAS_DEATH")
  (`PrimitiveComponent.SetCollisionEnabled` (`self.CapsuleComponent`) "NoCollision")
  (`CharacterMovementComponent.DisableMovement` (`self.CharacterMovement`)))

(event `AttackStyle Server`
  (params (`HeavyAttack?` :type Boolean))
  ;[0 0 0] Attack Style Server / Multicast
  (`self.AttackStyle Multi` `HeavyAttack?`))

(event `ChangeAnimState Server`
  (params (NewState :type "ECharAnimState Enum" :default "CAS_UNKNOWN"))
  ;[0 0 0] Change State Server / Multicast
  (`self.ChangeAnimState Multi` NewState))

(event `UpdateHealth Client`
  (params (Health :type "Float (double-precision)"))
  ;[0 0 0] Health Server / Client
  (bind _asbp_player_controller (cast `/Game/Blueprint/Characters/BP_PlayerController` (`GameplayStatics.GetPlayerController` 0)))
  (bind _gui_w (`/Game/Blueprint/Characters/BP_PlayerController.GUI_W` _asbp_player_controller)
    (:`then`
      (`/Game/Blueprint/Widgets/GUI_W.UpdateValues` _gui_w Health))
    (:`else`)))

(event `ChangeAnimState Multi`
  (params (NewState :type "ECharAnimState Enum" :default "CAS_UNKNOWN"))
  ;[0 0 0] Change State Server / Multicast
  (`self.ChangeAnimState` NewState))

(event `AttackStyle Multi`
  (params (`HeavyAttack?` :type Boolean))
  ;[0 0 0] Attack Style Server / Multicast
  (set `self.HeavyAttack?` `HeavyAttack?`))

(fn `ChangeAnimState`
  (params (NewState :type "ECharAnimState Enum" :default "CAS_UNKNOWN"))
  (`self.Animation`
    (:`then`
      (switch `ECharAnimState` (`local.NewState`)
        (:`CAS_IDLE`
          ;[0 0 0] Idle
          (`/Game/Blueprint/Characters/AnimBP_BaseCharacter.ChangeAnimStateTime` (`self.Animation`) "CAS_IDLE" 1.0 null)
          (set `CharacterMovementComponent.RotationRate` (struct :`Yaw` 360.0) (`self.CharacterMovement`))
          (set `self.MovementScale` 1.0))
        (:`CAS_ATTACK`
          ;[0 0 0] Attack
          (if (`|EnumInequality` (`CharacterMovementComponent.MovementMode` (`self.CharacterMovement`)) "MOVE_Falling")
            (if (`self.HeavyAttack?`)
              (`/Game/Blueprint/Characters/AnimBP_BaseCharacter.ChangeAnimStateTime` (`self.Animation`) "CAS_ATTACK" 1.0 "/Game/Mannequin/Animations/SwordShield_Sword_Attack_1.SwordShield_Sword_Attack_1")
              (else
                (`/Game/Blueprint/Characters/AnimBP_BaseCharacter.ChangeAnimStateTime` (`self.Animation`) "CAS_ATTACK" (`self.Recovery Duration`) "/Game/Mannequin/Animations/SwordShield_Sword_Attack_3.SwordShield_Sword_Attack_3")))
            (set `CharacterMovementComponent.RotationRate` (struct :`Yaw` 60.0) (`self.CharacterMovement`))
            (set `self.MovementScale` 0.1)
            (else
              (return))))
        (:`CAS_DAMAGE`
          ;[0 0 0] Damage
          (`/Game/Blueprint/Characters/AnimBP_BaseCharacter.ChangeAnimStateTime` (`self.Animation`) "CAS_DAMAGE" (`self.Recovery Duration`) "/Game/Mannequin/Animations/SwordShield_Impact_1.SwordShield_Impact_1"))
        (:`CAS_DEATH`
          ;[0 0 0] Death
          (`/Game/Blueprint/Characters/AnimBP_BaseCharacter.ChangeAnimStateTime` (`self.Animation`) "CAS_DEATH" 1.0 null)))
      (`parent.ChangeAnimState` (`local.NewState`)))
    (:`else`)))

(fn `ModifyDamage`
  (params (IncomingDamage :type "Float (double-precision)"))
  (returns (ReturnValue :type "Float (double-precision)"))
  (`self.ChangeAnimState Multi` "CAS_DAMAGE")
  (return IncomingDamage))

(fn `OnAttack`
  ;[0 0 0] Apply Damage to Enemy
  (for _array_element (`PrimitiveComponent.GetOverlappingActors` (`self.AttackRadius`) "/Script/Engine.Actor")
    (if (> (`self.GetDotProductTo` _array_element) 0.35)
      (if (`self.HeavyAttack?`)
        (`GameplayStatics.ApplyDamage` _array_element 100.0)
        (else
          (`GameplayStatics.ApplyDamage` _array_element (`self.Base Damage`)))))))

(fn `UserConstructionScript`)