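; Sword-and-shield enemy character with animated idle, run, attack, hit and death states and a floating health readout.
; Tick turns the color-coded health text toward the camera, removing it once dead.
; OnAttack damages player zero after a facing dot-product check; damage and death trigger animation changes through Server/Multicast events into AnimBP_BaseCharacter.
; Comments place behavior tree startup in Enemy_Controller; older timer-attack and AIMoveTo logic remains disconnected.
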(event `self.ReceiveTick`
  (params (DeltaSeconds :type "Float (single-precision)"))
  (bind _textrender_health (`self.TextRender_Health`))
  ;[0.4688 0 0.007142] Event Tick
  (if (`self.bDead`)
    (`/Engine/EditorBlueprintResources/StandardMacros.IsValid` _textrender_health
      (:`Is Valid`
        (`ActorComponent.K2_DestroyComponent` _textrender_health)))
    (else
      (`|ExecutionSequence`
        (:`then_0`
          (`self.UpdateHealthOnHead`))))))

(event `self.ReceiveBeginPlay`
  (bind _textrender_health (`self.TextRender_Health`))
  (`|ExecutionSequence`
    (:`then_0`
      (bind _asanim_bp_base_character (cast `/Game/Blueprint/Characters/AnimBP_BaseCharacter` (`SkeletalMeshComponent.GetAnimInstance` (`self.Mesh`))))
      (set `self.Animation` _asanim_bp_base_character))
    (:`then_1`
      (bind _asbp_avatar (cast `/Game/Blueprint/Characters/BP_Avatar` (`GameplayStatics.GetPlayerPawn` 0)))
      (set `self.As BP Avatar` _asbp_avatar))
    (:`then_2`
      (set `CharacterMovementComponent.MaxWalkSpeed` 500.0 (`self.CharacterMovement`)))
    (:`then_3`
      ;[0 0 0] Health Text Rotation
      (`SceneComponent.K2_SetWorldRotation` _textrender_health (`KismetMathLibrary.Conv_VectorToRotator` (- (`SceneComponent.K2_GetComponentLocation` (`self.TextRender_Health`)) (`self.K2_GetActorLocation` (`GameplayStatics.GetPlayerCameraManager` 0)))) false false :!label _label)
      (`TextRenderComponent.SetXScale` _textrender_health -1.0)
      (`TextRenderComponent.K2_SetText` (`self.TextRender_Health`) (`|FormatText` "Health: {health}" (`KismetTextLibrary.Conv_IntToText` (`KismetMathLibrary.Round` (`self.GetHealth`)))))
      (if (>= (`self.GetHealth`) 75.0)
        (`TextRenderComponent.SetTextRenderColor` (`self.TextRender_Health`) (make `Color` 0 255))
        (elif (and (< (`self.GetHealth`) 75.0) (> (`self.GetHealth`) 35.0))
          (`TextRenderComponent.SetTextRenderColor` (`self.TextRender_Health`) (make `Color` 0 155 155))
          (elif (<= (`self.GetHealth`) 35.0)
            (`TextRenderComponent.SetTextRenderColor` (`self.TextRender_Health`) (make `Color` 0 0 255))))))))

(event `UpdateHealthOnHead`
  ;[0 0 0] Health Text Rotation
  (goto _label))

(event `AttackApply`
  ;[0.1 0.1 0.1] Enemy GiveDamage System (OLD // Based on Event Timer)
  (if (not (`self.bDead`))
    (for _array_element (`PrimitiveComponent.GetOverlappingActors` (`self.AttackRadius`) "/Game/Blueprint/Characters/BP_Avatar.BP_Avatar_C")
      (if (> (`self.GetDotProductTo` _array_element) 0.35)
        (`GameplayStatics.ApplyDamage` (`GameplayStatics.GetPlayerPawn` 0) 10.0)))))

(event `SetBehavior`
  (bind _returnvalue (`AIBlueprintHelperLibrary.GetAIController` self))
  ;[0.2909 0.1791 0.4844] Run Behaviour Tree (BT_Enemy) // OLD // It's in the Enemy_Controller
  (`/Engine/EditorBlueprintResources/StandardMacros.IsValid` _returnvalue
    (:`Is Valid`
      (`AIController.RunBehaviorTree` _returnvalue "/Game/Blueprint/AI/Enemy/BT_Enemy.BT_Enemy"))))

(event `self.OnAttack`
  ;[0.3231 0 0.016] Event On Attack
  (if (> (`self.GetDotProductTo` (`GameplayStatics.GetPlayerPawn` 0)) 0.3)
    (`GameplayStatics.ApplyDamage` (`GameplayStatics.GetPlayerPawn` 0) 20.0)))

(event `self.OnCharacterDied`
  ;[0.3229 0 0.01598] Event Character Died
  (`self.ChangeAnimState Server` "CAS_DEATH")
  (`PrimitiveComponent.SetCollisionEnabled` (`self.CapsuleComponent`) "NoCollision")
  (`CharacterMovementComponent.DisableMovement` (`self.CharacterMovement`)))

(event `ChangeAnimState Server`
  (params (NewState :type "ECharAnimState Enum" :default "CAS_UNKNOWN"))
  ;[0 0 0] Change State Server / Multicast
  (`self.ChangeAnimState Multi` NewState))

(event `ChangeAnimState Multi`
  (params (NewState :type "ECharAnimState Enum" :default "CAS_UNKNOWN"))
  ;[0 0 0] Change State Server / Multicast
  (`self.ChangeAnimState` NewState))

(fn `ChangeAnimState`
  (params (NewState :type "ECharAnimState Enum" :default "CAS_UNKNOWN"))
  (`self.Animation`
    (:`then`
      (switch `ECharAnimState` (`local.NewState`)
        (:`CAS_IDLE`
          (`/Game/Blueprint/Characters/AnimBP_BaseCharacter.ChangeAnimStateTime` (`self.Animation`) "CAS_IDLE" 1.0 "/Game/Mannequin/Animations/SwordShield_Idle_2.SwordShield_Idle_2"))
        (:`CAS_RUN`
          (`/Game/Blueprint/Characters/AnimBP_BaseCharacter.ChangeAnimStateTime` (`self.Animation`) "CAS_RUN" 1.0 "/Game/Mannequin/Animations/SwordShield_Run.SwordShield_Run"))
        (:`CAS_ATTACK`
          (`/Game/Blueprint/Characters/AnimBP_BaseCharacter.ChangeAnimStateTime` (`self.Animation`) "CAS_ATTACK" 1.0 "/Game/Mannequin/Animations/SwordShield_Sword_Attack_3.SwordShield_Sword_Attack_3"))
        (:`CAS_DAMAGE`
          (`/Game/Blueprint/Characters/AnimBP_BaseCharacter.ChangeAnimStateTime` (`self.Animation`) "CAS_DAMAGE" 1.0 "/Game/Mannequin/Animations/SwordShield_Impact_1.SwordShield_Impact_1"))
        (:`CAS_DEATH`
          (`/Game/Blueprint/Characters/AnimBP_BaseCharacter.ChangeAnimStateTime` (`self.Animation`) "CAS_DEATH" 0.5 "/Game/Mannequin/Animations/SwordShield_Death_2.SwordShield_Death_2")))
      (`parent.ChangeAnimState` (`local.NewState`)))
    (:`else`
      (`KismetSystemLibrary.PrintString` "BP_Enemy - Animation is NOT VALID!" true true (struct :`R` 1.0 :`G` 0.012242 :`A` 1.0) 5.0))))

(fn `ModifyDamage`
  (params (IncomingDamage :type "Float (double-precision)"))
  (returns (ReturnValue :type "Float (double-precision)"))
  (`self.ChangeAnimState Server` "CAS_DAMAGE")
  (return IncomingDamage))

(fn `UpdateWalkSpeed`
  (params (`Max Walk Speed` :type "Float (double-precision)" :default 500.0))
  (set `CharacterMovementComponent.MaxWalkSpeed` `Max Walk Speed` (`self.CharacterMovement`)))

(fn `UserConstructionScript`)