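; BP_COAGameMode is a multiplayer game mode that handles player indexing on login and spawn point selection.
; On PostLogin, it copies LastPlayerIndex into the BP_COAPlayerState's PlayerIndex, then increments that PlayerIndex, leaving LastPlayerIndex itself unchanged.
; ChoosePlayerStart ignores that index, instead using the player's position in the GameState PlayerArray, wrapped by modulo over all PlayerStart actors.
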(event `self.K2_PostLogin`
  (params (NewPlayer :type "PlayerController Object Reference"))
  (bind _asbp_coaplayer_state (cast `/Game/Blueprint/Multiplayer/BP_COAPlayerState` (`Controller.PlayerState` NewPlayer)))
  (bind _output_get (set `/Game/Blueprint/Multiplayer/BP_COAPlayerState.PlayerIndex` (`self.Last Player Index`) _asbp_coaplayer_state))
  (`/Engine/EditorBlueprintResources/StandardMacros.IncrementInt` _output_get))

(fn `ChoosePlayerStart`
  (params (Player :type "Controller Object Reference"))
  (returns (ReturnValue :type "Actor Object Reference"))
  (bind _outactors (`GameplayStatics.GetAllActorsOfClass` "/Script/Engine.PlayerStart"))
  (return (`|GetArrayItem` _outactors (mod (`KismetArrayLibrary.Array_Find` (`GameStateBase.PlayerArray` (`GameplayStatics.GetGameState`)) (`Controller.PlayerState` Player)) (`KismetArrayLibrary.Array_Length` _outactors)))))

(fn `UserConstructionScript`)