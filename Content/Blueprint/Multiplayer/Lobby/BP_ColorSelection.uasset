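; Lobby color selection actor that sets a player's body color when their BP_Avatar overlaps it.
; The construction script maps ColorIndex to blue, red, yellow or green and styles the TextRender label to match.
; On overlap, it tints the avatar's mesh, stores the color in the game instance's PlayerSettings and passes those settings to the avatar's SendPlayerSettingsServer, with no local-player check.
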(event `self.ReceiveBeginPlay`)

(event `self.ReceiveActorBeginOverlap`
  (params (OtherActor :type "Actor Object Reference"))
  (bind _asbp_avatar (cast `/Game/Blueprint/Characters/BP_Avatar` OtherActor))
  (`MeshComponent.SetVectorParameterValueOnMaterials` (`Character.Mesh` _asbp_avatar) "BodyColor" (`KismetMathLibrary.Conv_LinearColorToVector` (`self.Color`)))
  (bind _asbp_coagame_instance (cast `/Game/Blueprint/Multiplayer/BP_COAGameInstance` (`GameplayStatics.GetGameInstance`)))
  (bind (_playersettings_displayname _playersettings_costumecolor _playersettings_weapontype) (break `/Game/Blueprint/Multiplayer/S_PlayerSettings` (`/Game/Blueprint/Multiplayer/BP_COAGameInstance.PlayerSettings` _asbp_coagame_instance)))
  (bind _output_get (set `/Game/Blueprint/Multiplayer/BP_COAGameInstance.PlayerSettings` (make `/Game/Blueprint/Multiplayer/S_PlayerSettings` _playersettings_displayname (`self.Color`) _playersettings_weapontype) _asbp_coagame_instance))
  (`/Game/Blueprint/Characters/BP_Avatar.SendPlayerSettings Server` _asbp_avatar _output_get))

(fn `UserConstructionScript`
  (`|ExecutionSequence`
    (:`then_0`
      (switch `int` (`self.ColorIndex`)
        (:`0`
          (set `self.Color` (`self.Blue`)))
        (:`1`
          (set `self.Color` (`self.Red`)))
        (:`2`
          (set `self.Color` (`self.Yellow`)))
        (:`3`
          (set `self.Color` (`self.Green`)))))
    (:`then_1`
      ;[0 0 0] Define Colors
      (if (== (`self.Color`) (`self.Blue`))
        (`TextRenderComponent.K2_SetText` (`self.TextRender`) (`self.BlueText`))
        (`TextRenderComponent.SetTextRenderColor` (`self.TextRender`) (`KismetMathLibrary.Conv_LinearColorToColor` (`self.Blue`)))
        (elif (== (`self.Color`) (`self.Red`))
          (`TextRenderComponent.K2_SetText` (`self.TextRender`) (`self.Red Text`))
          (`TextRenderComponent.SetTextRenderColor` (`self.TextRender`) (`KismetMathLibrary.Conv_LinearColorToColor` (`self.Red`)))
          (elif (== (`self.Color`) (`self.Yellow`))
            (`TextRenderComponent.K2_SetText` (`self.TextRender`) (`self.Yellow Text`))
            (`TextRenderComponent.SetTextRenderColor` (`self.TextRender`) (`KismetMathLibrary.Conv_LinearColorToColor` (`self.Yellow`)))
            (elif (== (`self.Color`) (`self.Green`))
              (`TextRenderComponent.K2_SetText` (`self.TextRender`) (`self.Green Text`))
              (`TextRenderComponent.SetTextRenderColor` (`self.TextRender`) (`KismetMathLibrary.Conv_LinearColorToColor` (`self.Green`))))))))))