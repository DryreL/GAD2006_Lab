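; A lobby weapon selection actor that sets a player's weapon type when their avatar walks into it.
; The construction script sets its text render label to match the configured weapon type: melee, sword or magic.
; On overlap with a BP_Avatar, it writes that type into the game instance's PlayerSettings, then changes the avatar's weapon through a multicast call.
; The overlap has no authority or local-player check before either step.
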(event `self.ReceiveBeginPlay`)

(event `self.ReceiveActorBeginOverlap`
  (params (OtherActor :type "Actor Object Reference"))
  (bind _weapon_type (`self.Weapon Type`))
  (bind _asbp_avatar (cast `/Game/Blueprint/Characters/BP_Avatar` OtherActor))
  (bind _asbp_coagame_instance (cast `/Game/Blueprint/Multiplayer/BP_COAGameInstance` (`GameplayStatics.GetGameInstance`)))
  (bind (_playersettings_displayname _playersettings_costumecolor) (break `/Game/Blueprint/Multiplayer/S_PlayerSettings` (`/Game/Blueprint/Multiplayer/BP_COAGameInstance.PlayerSettings` _asbp_coagame_instance)))
  (set `/Game/Blueprint/Multiplayer/BP_COAGameInstance.PlayerSettings` (make `/Game/Blueprint/Multiplayer/S_PlayerSettings` _playersettings_displayname _playersettings_costumecolor _weapon_type) _asbp_coagame_instance)
  (`/Game/Blueprint/Characters/BP_Avatar.ChangeWeaponType Multicast` _asbp_avatar _weapon_type))

(fn `UserConstructionScript`
  (switch `/Game/Blueprint/Multiplayer/E_WeaponType` (`self.Weapon Type`)
    (:`NewEnumerator0`
      (`TextRenderComponent.K2_SetText` (`self.TextRender`) (`self.Text - Melee`)))
    (:`NewEnumerator1`
      (`TextRenderComponent.K2_SetText` (`self.TextRender`) (`self.Text - Sword`)))
    (:`NewEnumerator2`
      (`TextRenderComponent.K2_SetText` (`self.TextRender`) (`self.Text - Magic`)))))