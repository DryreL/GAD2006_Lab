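; BP_Hanging_Trap is a hanging physics trap that the player can cut loose to damage enemies.
; A looping timer and a delay drive the PhysicsConstraint's angular orientation target between a value and its negation to produce swinging.
; When a BP_Avatar in its attack state begins overlapping the Box, the Sphere simulates physics, the Cable detaches and the constraint breaks.
; Any Sphere hit on a BP_Enemy applies damage.
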(event `self.ReceiveBeginPlay`
  (`KismetSystemLibrary.K2_SetTimerDelegate` (delegate `Angular`) 1.0 true))

(event `Angular`
  (`PhysicsConstraintComponent.SetAngularOrientationTarget` (`self.PhysicsConstraint`) (`self.In Pos Target`))
  (`KismetSystemLibrary.Delay` 1.0)
  (`PhysicsConstraintComponent.SetAngularOrientationTarget` (`self.PhysicsConstraint`) (* (`self.In Pos Target`) -1.0)))

(event `self.Sphere.OnComponentHit`
  (params (HitComponent :type "PrimitiveComponent Object Reference") (OtherActor :type "Actor Object Reference") (OtherComp :type "PrimitiveComponent Object Reference") (NormalImpulse :type "Vector Structure") (Hit :type "HitResult Structure (by ref)"))
  (bind _asbp_enemy (cast `/Game/Blueprint/BP_Enemy` (`.HitActor` (`GameplayStatics.BreakHitResult` Hit))))
  (`GameplayStatics.ApplyDamage` _asbp_enemy 100.0))

(event `self.Box.OnComponentBeginOverlap`
  (params (OverlappedComponent :type "PrimitiveComponent Object Reference") (OtherActor :type "Actor Object Reference") (OtherComp :type "PrimitiveComponent Object Reference") (OtherBodyIndex :type Integer) (bFromSweep :type Boolean) (SweepResult :type "HitResult Structure (by ref)"))
  (bind _asbp_avatar (cast `/Game/Blueprint/BP_Avatar` OtherActor))
  (if (`|EnumEquality` (`COABaseCharacter.AnimState` _asbp_avatar) "CAS_ATTACK")
    (`PrimitiveComponent.SetSimulatePhysics` (`self.Sphere`) true)
    (set `CableComponent.bAttachEnd` false (`self.Cable`))
    (`PhysicsConstraintComponent.BreakConstraint` (`self.PhysicsConstraint`))
    (`PhysicsConstraintComponent.BreakConstraint` (`self.PhysicsConstraint`))))

(fn `UserConstructionScript`)