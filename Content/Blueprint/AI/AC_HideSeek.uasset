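; AI controller for hide-and-seek characters that feeds PawnSensing sight and hearing into the Blackboard.
; When the controlled pawn is not the seeker, any seen BP_HideSeekChar becomes VisibleEnemy and its position is written to MoveLocation.
; Heard noises set NoiseLocation for any role, and a short retriggerable delay clears it once noise stops.
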(event `self.PawnSensing.OnSeePawn`
  (params (Pawn :type "Pawn Object Reference"))
  (bind _asbp_hide_seek_char (cast `/Game/Blueprint/AI/BP_HideSeekChar` Pawn))
  (if (not (`/Game/Blueprint/AI/BP_HideSeekChar.IsSeeker` (cast `/Game/Blueprint/AI/BP_HideSeekChar` (`self.K2_GetPawn`) :!pure true)))
    (`BlackboardComponent.SetValueAsObject` (`AIBlueprintHelperLibrary.GetBlackboard` self) "VisibleEnemy" _asbp_hide_seek_char)
    (`BlackboardComponent.SetValueAsVector` (`AIBlueprintHelperLibrary.GetBlackboard` self) "MoveLocation" (`self.K2_GetActorLocation` _asbp_hide_seek_char))))

(event `self.PawnSensing.OnHearNoise`
  (params (Instigator :type "Pawn Object Reference") (Location :type "Vector Structure (by ref)") (Volume :type "Float (single-precision)"))
  (bind _returnvalue (`AIBlueprintHelperLibrary.GetBlackboard` self))
  (`BlackboardComponent.SetValueAsVector` _returnvalue "NoiseLocation" Location)
  (`KismetSystemLibrary.RetriggerableDelay` 0.5)
  (`BlackboardComponent.ClearValue` _returnvalue "NoiseLocation"))

(fn `UserConstructionScript`)