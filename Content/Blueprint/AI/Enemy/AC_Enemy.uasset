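; AI controller for enemies that runs the BT_Enemy behavior tree on possession and tracks the player through AI Perception.
; Sensing a "Player"-tagged actor cancels the lose-sight timer and sets HasLineOfSight and EnemyActor on the Blackboard.
; Any other perception update starts that timer, which clears both keys after the LineOfSightTimer delay.
; Older PawnSensing logic, including PatrolLocation updates, remains disconnected and never runs.
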(event `self.PawnSensing.OnSeePawn`
  (params (Pawn :type "Pawn Object Reference"))
  ;[0.1 0.1 0.1] OLD CODE // NOT WORKING
)

(event `self.ReceivePossess`
  (params (PossessedPawn :type "Pawn Object Reference"))
  ;[0.2098 0.05125 0.4844] Run Behaviour Tree
  (`self.RunBehaviorTree` "/Game/Blueprint/AI/Enemy/BT_Enemy.BT_Enemy"))

(event `self.PawnSensing.OnHearNoise`
  (params (Instigator :type "Pawn Object Reference") (Location :type "Vector Structure (by ref)") (Volume :type "Float (single-precision)"))
  ;[0.1 0.1 0.1] OLD CODE // NOT WORKING
)

(event `self.AIPerception.OnTargetPerceptionUpdated`
  (params (Actor :type "Actor Object Reference") (Stimulus :type "AIStimulus Structure"))
  (bind _blackboard (`self.Blackboard`))
  (if (and (`self.ActorHasTag` Actor "Player") (`.bSuccessfullySensed` (break `AIStimulus` Stimulus)))
    (`KismetSystemLibrary.K2_ClearAndInvalidateTimerHandle` (`self.EnemyTimer`))
    (`BlackboardComponent.SetValueAsBool` _blackboard (`self.HasLineOfSight`) true)
    (`BlackboardComponent.SetValueAsObject` _blackboard (`self.EnemyActor`) Actor)
    (else
      ;[0 0.2292 0.01272] Enemy Timer
      (bind _returnvalue (`KismetSystemLibrary.K2_SetTimerDelegate` (delegate `StartEnemyTimer`) (`self.LineOfSightTimer`)))
      (set `self.EnemyTimer` _returnvalue))))

(event `StartEnemyTimer`
  (bind _blackboard (`self.Blackboard`))
  ;[0 0.2292 0.01272] Enemy Timer
  (`BlackboardComponent.SetValueAsBool` _blackboard (`self.HasLineOfSight`) false)
  (`BlackboardComponent.SetValueAsObject` _blackboard (`self.EnemyActor`) null))

(fn `UserConstructionScript`)