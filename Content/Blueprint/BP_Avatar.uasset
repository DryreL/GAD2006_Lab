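; BP_Avatar is the player character Blueprint, turning attack input and player death into animation state changes.
; BeginPlay caches the AnimBP_BaseCharacter instance, which ChangeAnimState drives before calling its parent version.
; Attack only starts from idle while not falling and slows turning and movement, Idle restores both, and Run is blocked after death.
; ChangeState is an empty stub, and ModifyDamage passes damage through unchanged.
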(event `self.ReceiveBeginPlay`
  (bind _asanim_bp_avatar (cast `/Game/Mannequin/Animations/AnimBP_BaseCharacter` (`SkeletalMeshComponent.GetAnimInstance` (`self.Mesh`)))
    (:`then`
      (set `self.Animation` _asanim_bp_avatar)
      (`self.ChangeState` "CAS_IDLE"))
    (:`CastFailed`
      (`KismetSystemLibrary.PrintString` "Cast failed!" true true (struct :`R` 1.0 :`B` 0.005787 :`A` 1.0) 5.0))))

(event `self.ReceiveTick`
  (params (DeltaSeconds :type "Float (single-precision)")))

(event `InputAction|Attack`
  (params (Key :type "Key Structure"))
  (:`Pressed`
    (`self.ChangeAnimState` "CAS_ATTACK")))

(event `self.PlayerDied`
  (`self.ChangeAnimState` "CAS_DEATH"))

(fn `ChangeAnimState`
  (params (NewState :type "ECharAnimState Enum" :default "CAS_UNKNOWN"))
  (bind _animation (`self.Animation`)
    (:`then`
      (`KismetSystemLibrary.PrintString` (`|GetEnumeratorNameAsString` NewState))
      (switch `ECharAnimState` NewState
        (:`CAS_IDLE`
          (`COACharAnimInstance.ChangeAnimState` _animation "CAS_IDLE")
          (set `CharacterMovementComponent.RotationRate` (struct :`Yaw` 360.0) (`self.CharacterMovement`))
          (set `self.MovementScale` 1.0)
          (`parent.ChangeAnimState` NewState :!label _label))
        (:`CAS_RUN`
          (if (`|EnumInequality` (`COACharAnimInstance.AnimState` _animation) "CAS_DEATH")
            (`COACharAnimInstance.ChangeAnimState` _animation "CAS_RUN")
            (goto _label)))
        (:`CAS_ATTACK`
          (if (and (`|EnumEquality` (`COACharAnimInstance.AnimState` _animation) "CAS_IDLE") (`|EnumInequality` (`CharacterMovementComponent.MovementMode` (`self.CharacterMovement`)) "MOVE_Falling"))
            (`COACharAnimInstance.ChangeAnimState` _animation "CAS_ATTACK")
            (set `CharacterMovementComponent.RotationRate` (struct :`Yaw` 60.0) (`self.CharacterMovement`))
            (set `self.MovementScale` 0.1)
            (goto _label)))
        (:`CAS_DAMAGE`
          (`COACharAnimInstance.ChangeAnimState` _animation (`local.NewState`) :!label _label_2)
          (goto _label))
        (:`CAS_DEATH`
          (goto _label_2))))
    (:`else`
      (`KismetSystemLibrary.PrintString` "Get Animation - Cast Failed!" true true (struct :`R` 1.0 :`B` 0.005787 :`A` 1.0) 5.0))))

(fn `ChangeState`
  (params (Selection :type "ECharAnimState Enum" :default "CAS_IDLE")))

(fn `ModifyDamage`
  (params (IncomingDamage :type "Float (double-precision)"))
  (returns (ReturnValue :type "Float (double-precision)"))
  (return IncomingDamage))

(fn `UserConstructionScript`)