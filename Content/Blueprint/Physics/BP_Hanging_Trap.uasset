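; Hanging trap: a sphere on a cable that the player can cut loose to damage enemies.
; A looping timer drives the physics constraint's angular orientation target between opposite values to swing it.
; A hit from an attacking BP_Avatar enables sphere physics, detaches the cable end and breaks the constraint.
; Sphere hits damage BP_Enemy only within a narrow dot-product range, intended to detect a falling sphere.
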(event `self.ReceiveBeginPlay`
  ;[0 0 0] Harmonic movement
  (`PhysicsConstraintComponent.SetAngularOrientationTarget` (`self.PhysicsConstraint`) (`self.In Pos Target`))
  (`KismetSystemLibrary.K2_SetTimerDelegate` (delegate `AngularLoop`) 1.0 true))

(event `AngularLoop`
  ;[0 0 0] Harmonic movement
  (`PhysicsConstraintComponent.SetAngularOrientationTarget` (`self.PhysicsConstraint`) (`self.In Pos Target`))
  (`KismetSystemLibrary.Delay` 1.0)
  (`PhysicsConstraintComponent.SetAngularOrientationTarget` (`self.PhysicsConstraint`) (* (`self.In Pos Target`) -1.0)))

(event `self.Sphere.OnComponentHit`
  (params (HitComponent :type "PrimitiveComponent Object Reference") (OtherActor :type "Actor Object Reference") (OtherComp :type "PrimitiveComponent Object Reference") (NormalImpulse :type "Vector Structure") (Hit :type "HitResult Structure (by ref)"))
  ;[0 0 0] Apply Damage
  (bind _asbp_enemy (cast `/Game/Blueprint/Characters/BP_Enemy` (`.HitActor` (`GameplayStatics.BreakHitResult` Hit))))
  (bind _returnvalue (`self.GetDotProductTo` _asbp_enemy))
  ;;[1 0.4686 0.2874] Return true if only sphere falls down
  (`KismetSystemLibrary.PrintString` (`KismetStringLibrary.Concat_StrStr` "Dot Product Value: " (`KismetStringLibrary.Conv_DoubleToString` _returnvalue)) true true (struct :`R` 0.524273 :`B` 1.0 :`A` 1.0) 5.0)
  (if (`KismetMathLibrary.InRange_FloatFloat` _returnvalue 0.1 0.2)
    (`GameplayStatics.ApplyDamage` _asbp_enemy 100.0)))

(event `self.ReceiveHit`
  (params (MyComp :type "PrimitiveComponent Object Reference") (Other :type "Actor Object Reference") (OtherComp :type "PrimitiveComponent Object Reference") (bSelfMoved :type Boolean) (HitLocation :type "Vector Structure") (HitNormal :type "Vector Structure") (NormalImpulse :type "Vector Structure") (Hit :type "HitResult Structure (by ref)"))
  ;[0 0 0] Cut the rope
  ;;[1 0.4686 0.2874] Return true if player attacks
  (bind _asbp_avatar (cast `/Game/Blueprint/Characters/BP_Avatar` Other))
  (if (`|EnumEquality` (`COABaseCharacter.AnimState` _asbp_avatar) "CAS_ATTACK")
    (`PrimitiveComponent.SetSimulatePhysics` (`self.Sphere`) true)
    (set `CableComponent.bAttachEnd` false (`self.Cable`))
    (`PhysicsConstraintComponent.BreakConstraint` (`self.PhysicsConstraint`))))

(fn `UserConstructionScript`)