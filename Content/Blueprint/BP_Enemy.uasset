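; BP_Enemy is an enemy Blueprint that relays animation state changes to its animation Blueprint.
; On BeginPlay it caches the mesh's AnimBP_BaseCharacter instance.
; ChangeAnimState calls the parent version and forwards the new state to that instance, only while the instance is valid.
; ModifyDamage switches to the damage state and returns incoming damage unchanged.
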(event `self.ReceiveBeginPlay`
  (bind _asanim_bp_avatar (cast `/Game/Mannequin/Animations/AnimBP_BaseCharacter` (`SkeletalMeshComponent.GetAnimInstance` (`self.Mesh`))))
  (set `self.Animation` _asanim_bp_avatar))

(fn `ChangeAnimState`
  (params (NewState :type "ECharAnimState Enum" :default "CAS_UNKNOWN"))
  (`self.Animation`
    (:`then`
      (`parent.ChangeAnimState` NewState)
      (`COACharAnimInstance.ChangeAnimState` (`self.Animation`) NewState))
    (:`else`)))

(fn `ModifyDamage`
  (params (IncomingDamage :type "Float (double-precision)"))
  (returns (ReturnValue :type "Float (double-precision)"))
  (`self.ChangeAnimState` "CAS_DAMAGE")
  (return IncomingDamage))

(fn `UserConstructionScript`)